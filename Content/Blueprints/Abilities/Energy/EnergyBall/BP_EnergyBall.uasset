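; BP_EnergyBall is an energy ball ability actor that explodes after a timed lifetime.
; BeginPlay starts a timer for the pre-explosion lifetime, with OnPreExplosionLifetimeExpired as the apparent callback into Explode.
; Explode sets the post-explosion lifespan, deactivates the VFX and prints a debug string.
; It has no damage or overlap logic.
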(event `self.ReceiveBeginPlay`
  (`KismetSystemLibrary.K2_SetTimerDelegate` (`|CreateDelegate` :!event `OnPreExplosionLifetimeExpired`) (`self.PreExplosionLifetime`)))

(fn `Explode`
  (`self.SetLifeSpan` (`self.PostExplosionLifetime`))
  (`ActorComponent.Deactivate` (`self.VFX`))
  (`KismetSystemLibrary.PrintString` "EXPLODE"))

(fn `OnPreExplosionLifetimeExpired`
  (`self.Explode`))

(fn `UserConstructionScript`)