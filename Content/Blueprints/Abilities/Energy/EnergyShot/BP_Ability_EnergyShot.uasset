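; Gameplay ability for an energy shot fired from the left hand, repeatable while active.
; Activation plays the firing montage and immediately line traces from the owner's eyes along control rotation, passing the hit to the energy shot gameplay cue without applying damage itself.
; After the montage, a short delay opens an input window: pressed or held input fires again, while a timeout ends the ability.
; GetEnergyShotStartLocation is an unused stub returning zero.
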(event `self.K2_ActivateAbility`
  (bind _timeouttask (`self.TimeoutTask`))
  (bind _asynctaskproxy (`AbilityTask_PlayMontageAndWait.CreatePlayMontageAndWaitProxy` "None" "/Game/Blueprints/Abilities/Energy/EnergyShot/Montage_EnergyShot_LeftHand.Montage_EnergyShot_LeftHand" 0.625 "Loop" :!label _label)
    (:`then`
      (set `self.MontageTask` _asynctaskproxy)
      (`self.Shoot`))
    (:`OnCompleted`
      (`AbilityTask_WaitDelay.WaitDelay` 0.15 :!label _label_2
        (:`then`
          (`AbilityTask_WaitInputPress.WaitInputPress` true
            (:`then`
              (bind _asynctaskproxy_2 (`AbilityTask_WaitDelay.WaitDelay` 1.5)
                (:`then`
                  (set `self.TimeoutTask` _asynctaskproxy_2))
                (:`OnFinish`
                  (`KismetSystemLibrary.PrintString` "END")
                  (`self.K2_EndAbility`))))
            (:`OnPress`
              (`/Engine/EditorBlueprintResources/StandardMacros.IsValid` _timeouttask
                (:`Is Valid`
                  (`GameplayTask.EndTask` _timeouttask)
                  (set `self.TimeoutTask` null)
                  (goto _label))
                (:`Is Not Valid`
                  (goto _label))))))))
    (:`OnBlendOut`
      (goto _label_2))
    (:`OnInterrupted`
      (`KismetSystemLibrary.PrintString` "Hello"))
    (:`OnCancelled`
      (`self.K2_EndAbility`))))

(event `Shoot`
  (bind _cachedcharacterowner (`self.CachedCharacterOwner`))
  (bind _outlocation (`Actor.GetActorEyesViewPoint` _cachedcharacterowner))
  (bind _outhit (`KismetSystemLibrary.LineTraceSingleByProfile` _outlocation (+ _outlocation (* (`KismetMathLibrary.GetForwardVector` (`Pawn.GetControlRotation` _cachedcharacterowner)) 5000.0)) "None" false (`|MakeArray` _cachedcharacterowner :!type "Actor Object Reference")))
  (`self.K2_ExecuteGameplayCueWithParams` (struct :`TagName` "GameplayCue.Energy.Shot") (`GameplayCueFunctionLibrary.MakeGameplayCueParametersFromHitResult` _outhit)))

(fn `GetEnergyShotStartLocation`
  (returns (StartLocWorldSpace :type "Vector Structure"))
  (return (+ (0.0 0.0 0.0) (0.0 0.0 0.0))))