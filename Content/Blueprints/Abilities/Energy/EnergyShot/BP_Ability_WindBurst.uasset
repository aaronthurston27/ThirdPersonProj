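; Wind energy gameplay ability that fires on input release, blasting physics objects away in a cone.
; A long enough hold, off cooldown, adds an eye-trace shot that triggers a cue and applies a wind effect to the target, narrows the cone and applies CGE_WindShot to the owner.
; After the montage blends out, another press loops back for the next attack, while a short idle timeout ends the ability.
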(event `self.K2_ActivateAbility`
  (bind _timeouttask (`self.TimeoutTask`))
  (bind (_asynctaskproxy _timeheld) (`AbilityTask_WaitInputRelease.WaitInputRelease` true :!label _label)
    (:`OnRelease`
      (bind _asynctaskproxy_2 (`AbilityTask_PlayMontageAndWait.CreatePlayMontageAndWaitProxy` "None" "/Game/Blueprints/Abilities/Energy/EnergyShot/Montage_WindShot_LeftHand.Montage_WindShot_LeftHand" 0.625 "Loop")
        (:`then`
          (set `self.MontageTask` _asynctaskproxy_2)
          (if (`self.Should Use Windshot` _timeheld)
            ;[1 1 1] Add extra wind, smaller wind burst here in case player still needs to blast enemies away while shooting.
            (`self.Wind Shot`)
            (`self.Wind Burst` (`self.Wind Burst Length`) 35.0 40.0)
            (`self.BP_ApplyGameplayEffectToOwner` "/Game/Blueprints/Abilities/Energy/EnergyShot/CGE_WindShot.CGE_WindShot_C")
            (else
              (`self.Wind Burst` (`self.Wind Burst Length`) 50.0 40.0))))
        (:`OnBlendOut`
          (`AbilityTask_WaitDelay.WaitDelay` 0.15
            (:`then`
              (`AbilityTask_WaitInputPress.WaitInputPress` true
                (:`then`
                  (if (not (`self.IsAbilityInputPressed`))
                    (bind _asynctaskproxy_3 (`AbilityTask_WaitDelay.WaitDelay` 1.5)
                      (:`then`
                        (set `self.TimeoutTask` _asynctaskproxy_3))
                      (:`OnFinish`
                        (`self.K2_EndAbility`)))))
                (:`OnPress`
                  (`/Engine/EditorBlueprintResources/StandardMacros.IsValid` _timeouttask
                    (:`Is Valid`
                      (`GameplayTask.EndTask` _timeouttask)
                      (set `self.TimeoutTask` null)
                      (goto _label))
                    (:`Is Not Valid`
                      (goto _label))))))))
        (:`OnInterrupted`
          (`KismetSystemLibrary.PrintString` "Hello"))
        (:`OnCancelled`
          (`self.K2_EndAbility`))))))

(event `self.K2_OnEndAbility`
  (params (bWasCancelled :type Boolean))
  (bind _timeouttask (`self.TimeoutTask`))
  (bind _montagetask (`self.MontageTask`))
  (`/Engine/EditorBlueprintResources/StandardMacros.IsValid` _timeouttask
    (:`Is Valid`
      (`GameplayTask.EndTask` _timeouttask))
    (:`Is Not Valid`
      _))
  (`/Engine/EditorBlueprintResources/StandardMacros.IsValid` _montagetask
    (:`Is Valid`
      (`GameplayTask.EndTask` _montagetask))))

(fn `Should Use Windshot`
  (params (InputTimeHeld :type "Float (double-precision)"))
  (returns (CanWindshot :type Boolean))
  (return (and (>= InputTimeHeld (`self.EnergyShotTimeThreshold`)) (not (`GameplayTagAssetInterface.HasMatchingGameplayTag` (`self.GetAbilitySystemComponentFromActorInfo`) (struct :`TagName` "Element.Wind.Cooldown.WindShot"))))))

(fn `Wind Burst`
  (params (`Burst Length` :type "Float (double-precision)") (WidthAngle :type "Float (double-precision)" :default 45.0) (HeightAngle :type "Float (double-precision)" :default 1.0))
  (bind _cachedcharacterowner (`self.CachedCharacterOwner`))
  (bind _returnvalue (`TPPFunctionLibrary.GetAllOverlapsWithinCone` (`Actor.K2_GetActorLocation` _cachedcharacterowner) (`Pawn.GetControlRotation` _cachedcharacterowner) `Burst Length` WidthAngle HeightAngle (`|MakeArray` _cachedcharacterowner :!type "Actor Object Reference")))
  (for _array_element _returnvalue
    (bind (_bblockinghit _binitialoverlap _time _distance _location _impactpoint _normal _impactnormal _physmat _hitactor) (`GameplayStatics.BreakHitResult` _array_element))
    (bind _returnvalue_2 (`Actor.GetComponentByClass` _hitactor "/Script/Engine.MeshComponent"))
    (`/Engine/EditorBlueprintResources/StandardMacros.IsValid` _returnvalue_2
      (:`Is Valid`
        (if (`SceneComponent.IsSimulatingPhysics` _returnvalue_2 "None")
          (`PrimitiveComponent.AddImpulseAtLocation` _returnvalue_2 (* (`KismetMathLibrary.NegateVector` _impactnormal) (* (`PrimitiveComponent.GetMass` _returnvalue_2) 900.0)) _impactpoint "None"))))))

(fn `Wind Shot`
  (bind _cachedcharacterowner (`self.CachedCharacterOwner`))
  (bind _outlocation (`Actor.GetActorEyesViewPoint` _cachedcharacterowner))
  (bind _outhit (`KismetSystemLibrary.LineTraceSingle` _outlocation (+ _outlocation (* (`KismetMathLibrary.GetForwardVector` (`Pawn.GetControlRotation` _cachedcharacterowner)) 5000.0)) "TraceTypeQuery3" false (`|MakeArray` _cachedcharacterowner :!type "Actor Object Reference")))
  (`self.K2_ExecuteGameplayCueWithParams` (struct :`TagName` "GameplayCue.Energy.Shot") (`GameplayCueFunctionLibrary.MakeGameplayCueParametersFromHitResult` _outhit))
  (bind (_bblockinghit _binitialoverlap _time _distance _location _impactpoint _normal _impactnormal _physmat _hitactor) (`GameplayStatics.BreakHitResult` _outhit))
  (`/Engine/EditorBlueprintResources/StandardMacros.IsValid` _hitactor
    (:`Is Valid`
      (bind _returnvalue (`Actor.GetComponentByClass` _hitactor "/Script/GameplayAbilities.AbilitySystemComponent"))
      (`/Engine/EditorBlueprintResources/StandardMacros.IsValid` _returnvalue
        (:`Is Valid`
          (`AbilitySystemComponent.BP_ApplyGameplayEffectToTarget` _returnvalue "/Game/Blueprints/Abilities/Energy/EnergyShot/GE_Element_WindShot.GE_Element_WindShot_C" _returnvalue 1.0 (make `GameplayEffectContextHandle`)))))))