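; Melee gameplay ability that plays an air or ground attack montage, chosen by whether the character is falling.
; It turns off physics rotation during root motion while the montage plays and restores it on blend out or ability end.
; Montage events pass their data to HandleMeleeTraceResult, which is empty here.
; Completion ends the ability, while interruption or cancellation cancels it.
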(event `self.K2_ActivateAbility`
  (bind (_asynctaskproxy _eventtag _eventdata) (`AT_PlayMontageAndWaitForEvent.PlayMontageAndWaitForEvent` "MeleeMontage" (select `bool` (`NavMovementComponent.IsFalling` (`Character.CharacterMovement` (`self.CachedCharacterOwner`))) :`false` (`self.Ground Melee Montage`) :`true` (`self.Air Melee Montage`)))
    (:`then`
      (set `CharacterMovementComponent.bAllowPhysicsRotationDuringAnimRootMotion` false (`ThirdPersonProjCharacter.GetThirdPersonMovementComponent` (`self.CachedCharacterOwner`))))
    (:`EventReceived`
      (`self.HandleMeleeTraceResult` _eventdata))
    (:`OnCompleted`
      (`self.K2_EndAbility`))
    (:`OnBlendOut`
      (set `CharacterMovementComponent.bAllowPhysicsRotationDuringAnimRootMotion` true (`ThirdPersonProjCharacter.GetThirdPersonMovementComponent` (`self.CachedCharacterOwner`))))
    (:`OnInterrupted`
      (`self.K2_CancelAbility` :!label _label))
    (:`OnCancelled`
      (goto _label))))

(event `self.K2_OnEndAbility`
  (params (bWasCancelled :type Boolean))
  (set `CharacterMovementComponent.bAllowPhysicsRotationDuringAnimRootMotion` true (`ThirdPersonProjCharacter.GetThirdPersonMovementComponent` (`self.CachedCharacterOwner`))))

(fn `HandleMeleeTraceResult`
  (params (EventData :type "GameplayEventData Structure")))