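; Wind jump gameplay ability that gives the character a jump, a charged high jump and a held glide.
; With the Wind Enhanced tag, a long enough hold boosts the jump on release and consumes one enhance stack; otherwise it jumps immediately.
; Holding input while airborne glides once descending, with zero gravity and a tick task easing vertical velocity logarithmically toward glide speed.
; Ending the ability restores gravity and jump velocity.
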(event `On Charge Jump`
  (`self.K2_EndAbility`))

(event `self.K2_ActivateAbility`
  (bind _cachedcharacterowner (`self.CachedCharacterOwner`))
  (bind _cachedcharacterowner_2 (`self.CachedCharacterOwner`))
  (bind _cachedcharacterowner_3 (`self.CachedCharacterOwner`))
  (bind _cachedcharacterowner_4 (`self.CachedCharacterOwner`))
  (bind _returnvalue (`ThirdPersonProjCharacter.GetThirdPersonMovementComponent` _cachedcharacterowner_3))
  (bind _returnvalue_2 (`GameplayTagAssetInterface.HasMatchingGameplayTag` (`self.GetAbilitySystemComponentFromActorInfo`) (struct :`TagName` "Element.Wind.Enhanced")))
  (bind _charactermovement (`Character.CharacterMovement` _cachedcharacterowner_3))
  (set `self.PrevGravityScale` (`CharacterMovementComponent.GravityScale` _returnvalue))
  (set `self.PrevJumpVelocity` (`CharacterMovementComponent.JumpZVelocity` _returnvalue))
  (set `CharacterMovementComponent.bNotifyApex` true _charactermovement)
  (switch `EMovementMode` (`CharacterMovementComponent.MovementMode` _charactermovement)
    (:`MOVE_Walking`
      (if _returnvalue_2 :!label _label
        (bind (_asynctaskproxy _timeheld) (`AbilityTask_WaitInputRelease.WaitInputRelease` true)
          (:`then`
            (set `self.Jump Charge Task` _asynctaskproxy)
            (add `Character.MovementModeChangedDelegate` _cachedcharacterowner_4 (`|CreateDelegate` :!event `Handle Movement Mode Changed`)))
          (:`OnRelease`
            (if (and (>= _timeheld (`self.WindJumpTime`)) _returnvalue_2)
              (set `CharacterMovementComponent.JumpZVelocity` (`self.WindJumpVelocity`) (`ThirdPersonProjCharacter.GetThirdPersonMovementComponent` (`self.CachedCharacterOwner`)))
              (`AbilitySystemComponent.RemoveActiveGameplayEffectBySourceEffect` (`ThirdPersonProjCharacter.TPPAbilitySystemComponent` _cachedcharacterowner_4) "/Game/Blueprints/Abilities/Wind/WindOrb/CGE_WindEnhance.CGE_WindEnhance_C" null 1))
            (`Character.Jump` _cachedcharacterowner_2)
            (add `ThirdPersonProjCharacter.OnJumpedEvent` _cachedcharacterowner_2 (`|CreateDelegate` :!event `On Charge Jump`))))
        (else
          (`Character.Jump` _cachedcharacterowner)
          (`AbilityTask_WaitInputRelease.WaitInputRelease` false
            (:`then`
              (add `Character.OnReachedJumpApex` (`self.CachedCharacterOwner`) (`|CreateDelegate` :!event `On Jump Apex Reached`)))
            (:`OnRelease`
              (`Character.StopJumping` _cachedcharacterowner)
              (`self.K2_EndAbility`))))))
    (:`MOVE_NavWalking`
      (goto _label))
    (:`MOVE_Falling`
      (`self.QueueGlide`))))

(event `QueueGlide`
  (bind (_returnvalue_x _returnvalue_y _returnvalue_z) (`KismetMathLibrary.BreakVector` (`Actor.GetVelocity` (`self.CachedCharacterOwner`))))
  (if (< _returnvalue_z 0.0)
    (`self.Start Gliding`)
    (else
      (add `Character.OnReachedJumpApex` (`self.CachedCharacterOwner`) (delegate `On Jump Apex Reached`))
      (bind _asynctaskproxy (`AbilityTask_WaitInputRelease.WaitInputRelease` false)
        (:`then`
          (set `self.GlideQueue` _asynctaskproxy))
        (:`OnRelease`
          (`self.K2_EndAbility`))))))

(event `On Jump Apex Reached`
  (bind _glidequeue (`self.GlideQueue`))
  (`/Engine/EditorBlueprintResources/StandardMacros.IsValid` _glidequeue
    (:`Is Valid`
      (`GameplayTask.EndTask` _glidequeue))
    (:`Is Not Valid`
      _))
  (if (`self.IsAbilityInputPressed`)
    (`self.Start Gliding`)
    (else
      (`self.K2_EndAbility`))))

(event `Start Gliding`
  (add `Character.MovementModeChangedDelegate` (`self.CachedCharacterOwner`) (`|CreateDelegate` :!event `Handle Movement Mode Changed`))
  (bind (_asynctaskproxy _deltatime) (`AT_Tick.AbilityTask_OnTick` "Glide Task")
    (:`then`
      (`AbilityTask_WaitInputRelease.WaitInputRelease` false
        (:`then`
          (set `CharacterMovementComponent.GravityScale` 0.0 (`ThirdPersonProjCharacter.GetThirdPersonMovementComponent` (`self.CachedCharacterOwner`))))
        (:`OnRelease`
          (`self.K2_EndAbility`))))
    (:`OnTick`
      (`self.TickCharacterGlideVelocity` _deltatime))))

(event `Handle Movement Mode Changed`
  (params (Character :type "Character Object Reference") (PrevMovementMode :type "EMovementMode Enum" :default "MOVE_None") (PreviousCustomMode :type Byte))
  (bind _jump_charge_task (`self.Jump Charge Task`))
  (switch `EMovementMode` PrevMovementMode
    (:`MOVE_Walking`
      (`/Engine/EditorBlueprintResources/StandardMacros.IsValid` _jump_charge_task :!label _label_2
        (:`Is Valid`
          (`GameplayTask.EndTask` _jump_charge_task))
        (:`Is Not Valid`
          _))
      (if (`|EnumEquality` (`CharacterMovementComponent.MovementMode` (`ThirdPersonProjCharacter.GetThirdPersonMovementComponent` (`self.CachedCharacterOwner`))) "MOVE_Falling")
        (`self.QueueGlide`)))
    (:`MOVE_NavWalking`
      (goto _label_2))
    (:`MOVE_Falling`
      (`self.K2_EndAbility`))))

(event `self.K2_OnEndAbility`
  (params (bWasCancelled :type Boolean))
  (bind _cachedcharacterowner (`self.CachedCharacterOwner`))
  (bind _returnvalue (`ThirdPersonProjCharacter.GetThirdPersonMovementComponent` _cachedcharacterowner))
  (remove `ThirdPersonProjCharacter.OnJumpedEvent` _cachedcharacterowner (`|CreateDelegate` :!event `On Charge Jump`))
  (remove `Character.MovementModeChangedDelegate` _cachedcharacterowner (`|CreateDelegate` :!event `Handle Movement Mode Changed`))
  (remove `Character.OnReachedJumpApex` _cachedcharacterowner (`|CreateDelegate` :!event `On Jump Apex Reached`))
  (set `CharacterMovementComponent.GravityScale` (`self.PrevGravityScale`) _returnvalue)
  (set `CharacterMovementComponent.JumpZVelocity` (`self.PrevJumpVelocity`) _returnvalue)
  (`parent.K2_OnEndAbility` false))

(fn `TickCharacterGlideVelocity`
  (params (DeltaTime :type "Float (double-precision)"))
  (bind (_returnvalue_x _returnvalue_y _returnvalue_z) (`KismetMathLibrary.BreakVector` (`Actor.GetVelocity` (`self.CachedCharacterOwner`))))
  (bind _returnvalue (- (`self.GlideZVelocity`) _returnvalue_z))
  (bind _returnvalue_2 (`KismetMathLibrary.Abs` _returnvalue))
  (set `MovementComponent.Velocity` (+ (* (`KismetMathLibrary.Vector_Up`) (select `bool` (< _returnvalue_2 2.0) :`false` (* (* (`KismetMathLibrary.Loge` _returnvalue_2) (`self.GlideDecelerationScale`)) (`local.DeltaTime`)) :`true` _returnvalue) (`KismetMathLibrary.SignOfFloat` _returnvalue)) (`Actor.GetVelocity` (`self.CachedCharacterOwner`))) (`Pawn.GetMovementComponent` (`self.CachedCharacterOwner`))))