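; Wind gameplay ability that casts a tornado in front of the owning character.
; On activation it snaps the character to the control yaw, locks movement-component rotation, and plays a slowed cast montage.
; A montage gameplay event spawns BP_Tornado at a set range along the character's flat forward vector.
; Montage completion or blend-out ends the ability, interruption cancels it, and ending re-enables rotation.
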(event `self.K2_ActivateAbility`
  (bind _cachedcharacterowner (`self.CachedCharacterOwner`))
  (bind _cachedcharacterowner_2 (`self.CachedCharacterOwner`))
  (bind (_returnvalue_roll _returnvalue_pitch _returnvalue_yaw) (`KismetMathLibrary.BreakRotator` (`Pawn.GetControlRotation` _cachedcharacterowner)))
  (`Actor.K2_SetActorRotation` _cachedcharacterowner (`KismetMathLibrary.MakeRotator` 0.0 0.0 _returnvalue_yaw) false)
  (set `CharacterMovementComponent.bUseControllerDesiredRotation` false (`ThirdPersonProjCharacter.GetThirdPersonMovementComponent` _cachedcharacterowner))
  (set `CharacterMovementComponent.bAllowPhysicsRotationDuringAnimRootMotion` false (`ThirdPersonProjCharacter.GetThirdPersonMovementComponent` (`self.CachedCharacterOwner`)))
  (`AT_PlayMontageAndWaitForEvent.PlayMontageAndWaitForEvent` "Cast Tornado" "/Game/Blueprints/Abilities/Wind/Tornado/Montage_CastTornado.Montage_CastTornado" (struct :`GameplayTags` (struct :`(TagName` "GameplayEvent.Wind.CastTornado"))) 0.55
    (:`EventReceived`
      (`|SpawnActorFromClass` "/Game/Blueprints/Abilities/Wind/Tornado/BP_Tornado.BP_Tornado_C" (`KismetMathLibrary.MakeTransform` (+ (`Actor.K2_GetActorLocation` _cachedcharacterowner_2) (* (`KismetMathLibrary.Vector_Normal2D` (`KismetMathLibrary.GetForwardVector` (`Actor.K2_GetActorRotation` _cachedcharacterowner_2))) (`self.Tornado Range`)))) "Undefined" "MultiplyWithRoot" null null))
    (:`OnCompleted`
      (`self.K2_EndAbility` :!label _label))
    (:`OnBlendOut`
      (goto _label))
    (:`OnInterrupted`
      (`self.K2_CancelAbility` :!label _label_2))
    (:`OnCancelled`
      (goto _label_2))))

(event `self.K2_OnEndAbility`
  (params (bWasCancelled :type Boolean))
  (bind _returnvalue (`ThirdPersonProjCharacter.GetThirdPersonMovementComponent` (`self.CachedCharacterOwner`)))
  (set `CharacterMovementComponent.bAllowPhysicsRotationDuringAnimRootMotion` true _returnvalue)
  (set `CharacterMovementComponent.bUseControllerDesiredRotation` true _returnvalue))