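; Wind Orb gameplay ability: shows a charging cue, then after a charge delay uses a short double-tap window to pick between throwing an orb and self-enhancing.
; A single press plays the throw montage, whose event spawns BP_WindOrb along control rotation with some forward character velocity added.
; A double tap plays the cast montage, whose event applies GE_Wind_Enhanced.
; Both cancel and block primary abilities only once chosen, committing cooldown on the montage event.
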(event `self.K2_ActivateAbility`
  ;[1 1 1] REMEMBER: Block primary abilities only when the throw montage starts. Set this to false. This is why we have set the cancel abilities with tag container.
  (`self.SetShouldBlockOtherAbilities` false)
  (`AbilityTask_WaitInputPress.WaitInputPress` true
    (:`OnPress`
      (`self.K2_AddGameplayCue` (struct :`TagName` "GameplayCue.Energy.BallCharging") (make `GameplayEffectContextHandle`))
      (`AbilityTask_WaitDelay.WaitDelay` (`self.ChargeDelay`)
        (:`OnFinish`
          (`AbilityTask_WaitInputPress.WaitInputPress` false
            (:`OnPress`
              (bind _asynctaskproxy (`AbilityTask_WaitDelay.WaitDelay` 0.35)
                (:`then`
                  (set `self.HoldInputTask` _asynctaskproxy)
                  (bind _asynctaskproxy_2 (`AbilityTask_WaitInputPress.WaitInputPress` false)
                    (:`then`
                      (set `self.DoubleTapTask` _asynctaskproxy_2))
                    (:`OnPress`
                      (`GameplayTask.EndTask` (`self.HoldInputTask`))
                      (bind _astppability_system_component (cast `TPPAbilitySystemComponent` (`self.GetAbilitySystemComponentFromActorInfo`)))
                      (`TPPAbilitySystemComponent.CancelAbilitiesByTag` _astppability_system_component (`BlueprintGameplayTagLibrary.MakeLiteralGameplayTagContainer` (struct :`GameplayTags` (struct :`(TagName` "GameplayAbility.PrimaryAbility")))))
                      (`TPPAbilitySystemComponent.BlockPrimaryAbilityInput` _astppability_system_component)
                      (`AT_PlayMontageAndWaitForEvent.PlayMontageAndWaitForEvent` "None" "/Game/Blueprints/Abilities/Wind/WindOrb/Animations/Montage_CastEnhance.Montage_CastEnhance" (struct :`GameplayTags` (struct :`(TagName` "GameplayEvent.Wind.CastEnhance"))) 1.15
                        (:`EventReceived`
                          (`self.BP_ApplyGameplayEffectToOwner` "/Game/Blueprints/Abilities/Wind/WindOrb/GE_Wind_Enhanced.GE_Wind_Enhanced_C" 1 2)
                          (`self.K2_CommitAbility`)
                          (`self.K2_CommitAbilityCooldown` true true))
                        (:`OnCompleted`
                          (bind _astppability_system_component_2 (cast `TPPAbilitySystemComponent` (`self.GetAbilitySystemComponentFromActorInfo`) :!label _label))
                          (`TPPAbilitySystemComponent.UnblockPrimaryAbilityInput` _astppability_system_component_2)
                          (`TPPAbilitySystemComponent.UnblockUltimateAbilityInput` _astppability_system_component_2)
                          (`self.K2_EndAbility`))
                        (:`OnBlendOut`
                          (goto _label))
                        (:`OnInterrupted`
                          (goto _label))
                        (:`OnCancelled`
                          (goto _label))))))
                (:`OnFinish`
                  (`GameplayTask.EndTask` (`self.DoubleTapTask`))
                  (bind _astppability_system_component_3 (cast `TPPAbilitySystemComponent` (`self.GetAbilitySystemComponentFromActorInfo`))
                    (:`then`
                      (`TPPAbilitySystemComponent.CancelAbilitiesByTag` _astppability_system_component_3 (`BlueprintGameplayTagLibrary.MakeLiteralGameplayTagContainer` (struct :`GameplayTags` (struct :`(TagName` "GameplayAbility.PrimaryAbility")))))
                      (`TPPAbilitySystemComponent.BlockPrimaryAbilityInput` _astppability_system_component_3))
                    (:`CastFailed`
                      _))
                  (`AT_PlayMontageAndWaitForEvent.PlayMontageAndWaitForEvent` "None" "/Game/Blueprints/Abilities/Wind/WindOrb/Animations/Montage_Throw.Montage_Throw" (struct :`GameplayTags` (struct :`(TagName` "GameplayEvent.Energy.SpawnBall"))) 1.5
                    (:`EventReceived`
                      (`self.SpawnEnergyBall`)
                      (`self.K2_RemoveGameplayCue` (struct :`TagName` "GameplayCue.Energy.BallCharging"))
                      (`self.K2_CommitAbility`)
                      (`self.K2_CommitAbilityCooldown` true true))
                    (:`OnCompleted`
                      (`self.K2_EndAbility` :!label _label_2))
                    (:`OnBlendOut`
                      (goto _label_2))
                    (:`OnInterrupted`
                      (goto _label_2))
                    (:`OnCancelled`
                      (goto _label_2))))))))))))

(event `self.K2_OnEndAbility`
  (params (bWasCancelled :type Boolean))
  (cast `TPPAbilitySystemComponent` (`self.GetAbilitySystemComponentFromActorInfo`))
  (`self.K2_RemoveGameplayCue` (struct :`TagName` "GameplayCue.Energy.BallCharging")))

(fn `SpawnEnergyBall`
  (bind _cachedcharacterowner (`self.CachedCharacterOwner`))
  (bind _cachedcharacterowner_2 (`self.CachedCharacterOwner`))
  (bind _returnvalue (`Pawn.GetControlRotation` _cachedcharacterowner_2))
  (bind _returnvalue_2 (`KismetMathLibrary.GetForwardVector` _returnvalue))
  (bind _returnvalue_3 (`|SpawnActorFromClass` "/Game/Blueprints/Abilities/Wind/WindOrb/BP_WindOrb.BP_WindOrb_C" (`KismetMathLibrary.MakeTransform` (+ (`SceneComponent.GetSocketLocation` (`Character.Mesh` _cachedcharacterowner_2) "ring_01_r") (* _returnvalue_2 (`self.SpawnForwardOffset`))) _returnvalue) "Undefined" "MultiplyWithRoot" _cachedcharacterowner null))
  (`/Engine/EditorBlueprintResources/StandardMacros.IsValid` _returnvalue_3
    (:`Is Valid`
      (`ProjectileMovementComponent.SetVelocityInLocalSpace` (`/Game/Blueprints/Abilities/Wind/WindOrb/BP_WindOrb.ProjectileMovement` _returnvalue_3) (`KismetMathLibrary.MakeVector` (+ (`self.LaunchForwardVelocity`) (* (`KismetMathLibrary.FMax` 0.0 (`KismetMathLibrary.Dot_VectorVector` (`Actor.GetVelocity` _cachedcharacterowner) _returnvalue_2)) 0.65)) 0.0 (* (`self.LaunchUpVelocity`) (`KismetMathLibrary.FMax` (`KismetMathLibrary.DegCos` (.pitch _returnvalue)))))))))