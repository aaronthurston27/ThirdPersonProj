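; Energy ball projectile for the Wind Orb ability that explodes into a hit effect and a physics impulse.
; A timer sets its fuse, shortened when the projectile stops, while a gameplay tag count above one on its ability system detonates it immediately.
; The explosion sphere-traces for pawns and physics bodies, then radially pushes physics-simulating meshes that pass a line-of-sight check against static world geometry.
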(event `self.ReceiveBeginPlay`
  (bind _returnvalue (`KismetSystemLibrary.K2_SetTimerDelegate` (`|CreateDelegate` :!event `OnPreExplosionLifetimeExpired`) (`self.ExplosionTime`)))
  (set `self.ExplosionHandle` _returnvalue))

(event `self.ProjectileMovement.OnProjectileStop`
  (params (ImpactResult :type "HitResult Structure (by ref)"))
  (bind _returnvalue (`KismetSystemLibrary.K2_SetTimerDelegate` (`|CreateDelegate` :!event `OnPreExplosionLifetimeExpired`) (`KismetMathLibrary.FMin` (- (`self.ExplosionTime`) (`KismetSystemLibrary.K2_GetTimerElapsedTimeHandle` (`self.ExplosionHandle`))) (`self.OnStopExplosionTime`))))
  (`KismetSystemLibrary.K2_ClearAndInvalidateTimerHandle` (`self.ExplosionHandle`))
  (set `self.ExplosionHandle` _returnvalue))

(event `self.TPPAbilitySystem.OnBaseGameplayTagCountChanged`
  (params (GameplayTag :type "GameplayTag Structure") (Count :type Integer))
  (if (> Count 1)
    (`self.Explode`)))

(event `self.TPPAbilitySystem.OnAnyGameplayTagCountChanged`
  (params (GameplayTag :type "GameplayTag Structure") (Count :type Integer)))

(fn `ApplyExplosionImpulse`
  (bind _returnvalue (`self.K2_GetActorLocation`))
  (bind _outhits (`KismetSystemLibrary.SphereTraceMultiForObjects` _returnvalue _returnvalue (`self.ExplosionRadius`) (`|MakeArray` "ObjectTypeQuery3" "ObjectTypeQuery4" :!type "EObjectTypeQuery Enum") true (`|MakeArray` self :!type "Actor Object Reference")))
  (for _array_element _outhits
    (`KismetSystemLibrary.PrintString` (`KismetSystemLibrary.GetDisplayName` (`.HitActor` (`GameplayStatics.BreakHitResult` _array_element))))
    (bind _returnvalue_2 (`self.GetComponentByClass` (`.HitActor` (`GameplayStatics.BreakHitResult` _array_element)) "/Script/Engine.MeshComponent"))
    (`/Engine/EditorBlueprintResources/StandardMacros.IsValid` _returnvalue_2
      (:`Is Valid`
        (bind (_outhit _returnvalue_3) (`KismetSystemLibrary.LineTraceSingleForObjects` (`.TraceStart` (`GameplayStatics.BreakHitResult` _array_element)) (`.ImpactPoint` (`GameplayStatics.BreakHitResult` _array_element)) (`|MakeArray` "ObjectTypeQuery1" :!type "EObjectTypeQuery Enum") true))
        (if _returnvalue_3
          _
          (elif (`SceneComponent.IsSimulatingPhysics` _returnvalue_2 "None")
            (`PhysicsObjectBlueprintLibrary.ApplyRadialImpulse` _returnvalue_2 (`.ImpactPoint` (`GameplayStatics.BreakHitResult` _array_element)) (`self.ExplosionRadius`) 60000.0 "RIF_Constant")))))))

(fn `Explode`
  (`PrimitiveComponent.SetCollisionEnabled` (`self.HitSphere`) "NoCollision")
  (`MovementComponent.StopMovementImmediately` (`self.ProjectileMovement`))
  (`KismetSystemLibrary.K2_ClearAndInvalidateTimerHandle` (`self.ExplosionHandle`))
  (`self.SetLifeSpan` (`self.PostExplosionLifetime`))
  (`ActorComponent.Deactivate` (`self.VFX`))
  (`NiagaraFunctionLibrary.SpawnSystemAtLocation` "/Game/sA_Projectilevfx_R1/Vfx/Fx/Niagara_Systems/NS_Hit7.NS_Hit7" (`self.K2_GetActorLocation`) (`self.K2_GetActorRotation`))
  (`KismetSystemLibrary.K2_ClearAndInvalidateTimerHandle` (`self.ExplosionHandle`))
  (`self.ApplyExplosionImpulse`))

(fn `OnPreExplosionLifetimeExpired`
  (`self.Explode`))

(fn `UserConstructionScript`)