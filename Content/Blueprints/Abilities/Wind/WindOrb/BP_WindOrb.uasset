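; Wind orb ability projectile that explodes into a burst of force, pushing nearby targets and physics objects.
; A fuse timer starts on BeginPlay and is capped to a shorter delay when the projectile stops.
; A base gameplay tag count above one also triggers Explode, which halts movement and swaps the orb VFX for a Niagara burst.
; A radius query sends impulses through AbilityForceTarget, or radial impulses to simulating meshes lacking that interface.
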(event `self.ReceiveBeginPlay`
  (bind _returnvalue (`KismetSystemLibrary.K2_SetTimerDelegate` (`|CreateDelegate` :!event `OnPreExplosionLifetimeExpired`) (`self.ExplosionTime`)))
  (set `self.ExplosionHandle` _returnvalue))

(event `self.ProjectileMovement.OnProjectileStop`
  (params (ImpactResult :type "HitResult Structure (by ref)"))
  (bind _returnvalue (`KismetSystemLibrary.K2_SetTimerDelegate` (`|CreateDelegate` :!event `OnPreExplosionLifetimeExpired`) (`KismetMathLibrary.FMin` (- (`self.ExplosionTime`) (`KismetSystemLibrary.K2_GetTimerElapsedTimeHandle` (`self.ExplosionHandle`))) (`self.OnStopExplosionTime`))))
  (`KismetSystemLibrary.K2_ClearAndInvalidateTimerHandle` (`self.ExplosionHandle`))
  (set `self.ExplosionHandle` _returnvalue))

(event `self.TPPAbilitySystem.OnBaseGameplayTagCountChanged`
  (params (GameplayTag :type "GameplayTag Structure") (Count :type Integer))
  (if (> Count 1)
    (`self.Explode`)))

(event `self.TPPAbilitySystem.OnAnyGameplayTagCountChanged`
  (params (GameplayTag :type "GameplayTag Structure") (Count :type Integer)))

(fn `DoExplosionTraces`
  (bind _sphere (`self.Sphere`))
  (bind _returnvalue (`TPPFunctionLibrary.GetOverlappingActorsInRadius` (`self.K2_GetActorLocation`) (`self.ExplosionRadius`) (`|MakeArray` self)))
  (for _array_element _returnvalue
    (bind (_bblockinghit _binitialoverlap _time _distance _location _impactpoint _normal _impactnormal _physmat _hitactor _hitcomponent _hitbonename) (`GameplayStatics.BreakHitResult` _array_element))
    (if (`KismetSystemLibrary.DoesImplementInterface` _hitactor "/Script/ThirdPersonProj.AbilityForceTarget")
      (bind _returnvalue_2 (message `AbilityForceTarget.CanApplyForceToTarget` _hitactor self _sphere _hitcomponent (struct) "None"))
      (if _returnvalue_2
        (message `AbilityForceTarget.AddImpulseToTarget` _hitactor self _sphere _hitcomponent (`KismetMathLibrary.NegateVector` (* _impactnormal (`self.ExplosionImpulseStrength`))) _impactpoint (struct) _hitbonename))
      (else
        (bind _asmesh_component (cast `MeshComponent` _hitcomponent))
        (if (`SceneComponent.IsSimulatingPhysics` _asmesh_component "None")
          (`PhysicsObjectBlueprintLibrary.ApplyRadialImpulse` _asmesh_component (`self.K2_GetActorLocation`) (`self.ExplosionRadius`) (`self.ExplosionImpulseStrength`) "RIF_Constant"))))))

(fn `Explode`
  (bind _vfx (`self.VFX`))
  (`PrimitiveComponent.SetCollisionEnabled` (`self.HitSphere`) "NoCollision")
  (`MovementComponent.StopMovementImmediately` (`self.ProjectileMovement`))
  (`KismetSystemLibrary.K2_ClearAndInvalidateTimerHandle` (`self.ExplosionHandle`))
  (`self.SetLifeSpan` (`self.PostExplosionLifetime`))
  (`ActorComponent.Deactivate` _vfx)
  (`SceneComponent.SetVisibility` _vfx false false)
  (`NiagaraFunctionLibrary.SpawnSystemAtLocation` "/Game/Blueprints/Abilities/Wind/WindOrb/FX/NS_WindOrb_Explosion.NS_WindOrb_Explosion" (`self.K2_GetActorLocation`) (`self.K2_GetActorRotation`))
  (`KismetSystemLibrary.K2_ClearAndInvalidateTimerHandle` (`self.ExplosionHandle`))
  (`self.DoExplosionTraces`))

(fn `OnPreExplosionLifetimeExpired`
  (`self.Explode`))

(fn `UserConstructionScript`)