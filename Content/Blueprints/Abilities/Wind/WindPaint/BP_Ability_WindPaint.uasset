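; Gameplay ability that lets the player paint a wind path in the world.
; On activation it blocks primary ability input, disables physics rotation during root motion, plays the control-wind montage and runs a user-confirmed wind-paint targeting actor.
; Confirmed target data creates the path, then a tick task updates it each frame, curving while the ability input is held.
; A one-frame delay before targeting prevents instant cancellation when right click is held.
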(event `self.K2_ActivateAbility`
  (bind _astppability_system_component (cast `TPPAbilitySystemComponent` (`self.GetAbilitySystemComponentFromActorInfo`)))
  (`TPPAbilitySystemComponent.BlockPrimaryAbilityInput` _astppability_system_component)
  (set `CharacterMovementComponent.bAllowPhysicsRotationDuringAnimRootMotion` false (`ThirdPersonProjCharacter.GetThirdPersonMovementComponent` (`self.CachedCharacterOwner`)))
  (`AT_PlayMontageAndWaitForEvent.PlayMontageAndWaitForEvent` "None" "/Game/Blueprints/Abilities/Wind/WindPaint/Montage_ControlWind.Montage_ControlWind"
    (:`then`
      ;[1 1 1] Wait for one frame here so we don't automatically cancel ability when right click held
      (`AbilityTask_WaitDelay.WaitDelay` 0.0
        (:`OnFinish`
          (bind (_asynctaskproxy _data) (`AbilityTask_WaitTargetData.WaitTargetData` "None" "UserConfirmed" "/Game/Blueprints/Abilities/Wind/WindPaint/BP_Targeting_WindPaint.BP_Targeting_WindPaint_C" 2000.0 (struct :`Name` "BlockOnlyStatic") false (`self.MakeTargetLocationInfoFromOwnerActor`) (struct) null (struct) true)
            (:`then`
              (set `self.TargetingTask` _asynctaskproxy))
            (:`ValidData`
              (bind (_returnvalue_startingposition _returnvalue_pathcenterpoint _returnvalue_windtraveldirection) (break `GameplayAbilityTargetData_WindPaint` (`self.GetTargetDataFromHandle` _data)))
              (`self.CreateWindPath` _returnvalue_startingposition _returnvalue_pathcenterpoint (`KismetMathLibrary.Conv_VectorToRotator` _returnvalue_windtraveldirection))
              (bind (_asynctaskproxy_2 _deltatime) (`AT_Tick.AbilityTask_OnTick` "Paint Wind")
                (:`then`
                  (set `self.Paint Wind Task` _asynctaskproxy_2))
                (:`OnTick`
                  (`self.SetWantsToCurvePath` (`self.IsAbilityInputPressed`))
                  (`self.UpdateWindPath` _deltatime))))
            (:`Cancelled`
              (`self.K2_EndAbility`))))))))

(event `self.K2_OnEndAbility`
  (params (bWasCancelled :type Boolean))
  (set `CharacterMovementComponent.bAllowPhysicsRotationDuringAnimRootMotion` true (`ThirdPersonProjCharacter.GetThirdPersonMovementComponent` (`self.CachedCharacterOwner`))))