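; Metal bat equipment ability for a big swing, with a held ready stance that leads into a swing on confirm input.
; Releasing input during the ready montage ends the ability; confirming cancels that release task, snaps the character to control rotation and plays the swing montage.
; When the swing completes or blends out, it returns to ready if input is still held, otherwise it ends.
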(event `self.K2_ActivateAbility`
  (`parent.K2_ActivateAbility`)
  (`self.Enter Bat Ready`))

(event `Enter Bat Ready`
  (bind _canceltask (`self.CancelTask`))
  (set `CharacterMovementComponent.bAllowPhysicsRotationDuringAnimRootMotion` true (`ThirdPersonProjCharacter.GetThirdPersonMovementComponent` (`self.CachedCharacterOwner`)))
  (`AbilityTask_PlayMontageAndWait.CreatePlayMontageAndWaitProxy` "None" "/Game/Blueprints/Items/Bat_Metal/Anim/Bat_Ready.Bat_Ready" 1.25
    (:`then`
      (`AT_WaitConfirmInput.WaitConfirmInput`
        (:`then`
          (bind _asynctaskproxy (`AbilityTask_WaitInputRelease.WaitInputRelease` true)
            (:`then`
              (set `self.CancelTask` _asynctaskproxy))
            (:`OnRelease`
              (`self.K2_EndAbility`))))
        (:`OnConfirm`
          (`self.Swing`)
          (`/Engine/EditorBlueprintResources/StandardMacros.IsValid` _canceltask
            (:`Is Valid`
              (`GameplayTask.EndTask` _canceltask)
              (set `self.CancelTask` null))))))
    (:`OnCancelled`
      (`self.K2_EndAbility`))))

(event `Swing`
  (bind _cachedcharacterowner (`self.CachedCharacterOwner`))
  (`self.MontageStop` -1.0)
  (`Actor.K2_SetActorRotation` _cachedcharacterowner (`Pawn.GetControlRotation` _cachedcharacterowner) false)
  (set `CharacterMovementComponent.bAllowPhysicsRotationDuringAnimRootMotion` true (`ThirdPersonProjCharacter.GetThirdPersonMovementComponent` _cachedcharacterowner))
  (bind _asynctaskproxy (`AT_PlayMontageAndWaitForEvent.PlayMontageAndWaitForEvent` "None" "/Game/Blueprints/Items/Bat_Metal/Anim/Bat_Swing.Bat_Swing")
    (:`OnCompleted`
      (if (`self.IsAbilityInputPressed`) :!label _label
        (`GameplayTask.EndTask` _asynctaskproxy)
        (`self.Enter Bat Ready`)
        (else
          (`self.K2_EndAbility`))))
    (:`OnBlendOut`
      (goto _label))
    (:`OnInterrupted`
      (`self.K2_EndAbility` :!label _label_2))
    (:`OnCancelled`
      (goto _label_2))))

(event `self.K2_OnEndAbility`
  (params (bWasCancelled :type Boolean))
  (set `CharacterMovementComponent.bAllowPhysicsRotationDuringAnimRootMotion` true (`ThirdPersonProjCharacter.GetThirdPersonMovementComponent` (`self.CachedCharacterOwner`))))