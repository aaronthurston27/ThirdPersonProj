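; Gameplay ability for the metal bat equipment: a hold-to-ready, release-to-swing attack.
; Activation plays the ready montage and waits for input release, with a cancel task that can end the ability until the swing starts.
; When the swing montage blends out or completes, it returns to ready if input is pressed, otherwise it ends.
; Physics rotation during root motion is disabled while readied and restored on swing or ability end.
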(event `self.K2_ActivateAbility`
  (`parent.K2_ActivateAbility`)
  (`self.Enter Bat Ready`))

(event `Enter Bat Ready`
  (bind _canceltask (`self.CancelTask`))
  (set `CharacterMovementComponent.bAllowPhysicsRotationDuringAnimRootMotion` false (`ThirdPersonProjCharacter.GetThirdPersonMovementComponent` (`self.CachedCharacterOwner`)))
  (`AbilityTask_PlayMontageAndWait.CreatePlayMontageAndWaitProxy` "None" "/Game/Blueprints/Items/Bat_Metal/Anim/Bat_Ready.Bat_Ready" 1.25
    (:`then`
      (`AbilityTask_WaitInputRelease.WaitInputRelease` true
        (:`then`
          (bind _asynctaskproxy (`AbilityTask_WaitCancel.WaitCancel`)
            (:`then`
              (set `self.CancelTask` _asynctaskproxy))
            (:`OnCancel`
              (`self.K2_EndAbility`))))
        (:`OnRelease`
          (`self.Swing`)
          (`/Engine/EditorBlueprintResources/StandardMacros.IsValid` _canceltask
            (:`Is Valid`
              (`GameplayTask.EndTask` _canceltask)
              (set `self.CancelTask` null))))))
    (:`OnInterrupted`
      (`self.K2_EndAbility` :!label _label))
    (:`OnCancelled`
      (goto _label))))

(event `Swing`
  (`self.MontageStop` -1.0)
  (set `CharacterMovementComponent.bAllowPhysicsRotationDuringAnimRootMotion` true (`ThirdPersonProjCharacter.GetThirdPersonMovementComponent` (`self.CachedCharacterOwner`)))
  (bind _asynctaskproxy (`AT_PlayMontageAndWaitForEvent.PlayMontageAndWaitForEvent` "None" "/Game/Blueprints/Items/Bat_Metal/Anim/Bat_Swing.Bat_Swing")
    (:`OnCompleted`
      (if (`self.IsAbilityInputPressed`) :!label _label_2
        (`GameplayTask.EndTask` _asynctaskproxy)
        (`self.Enter Bat Ready`)
        (else
          (`self.K2_EndAbility`))))
    (:`OnBlendOut`
      (goto _label_2))
    (:`OnInterrupted`
      (`self.K2_EndAbility` :!label _label_3))
    (:`OnCancelled`
      (goto _label_3))))

(event `self.K2_OnEndAbility`
  (params (bWasCancelled :type Boolean))
  (set `CharacterMovementComponent.bAllowPhysicsRotationDuringAnimRootMotion` true (`ThirdPersonProjCharacter.GetThirdPersonMovementComponent` (`self.CachedCharacterOwner`))))